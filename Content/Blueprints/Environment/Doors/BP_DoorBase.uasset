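; Base door actor that swings open when a ThirdPersonCharacter enters its trigger box and closes when it leaves.
; A timeline drives DoorRotator's yaw up to MaxDoorOpenAngle, playing forward to open and in reverse to close, then sets IsOpen from its direction.
; InProgress drops open or close requests made mid-swing, without queuing them.
; The construction script pre-rotates the door when IsOpen is set.
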(event `self.Box.OnComponentBeginOverlap`
  (params (OverlappedComponent :type "PrimitiveComponent Object Reference") (OtherActor :type "Actor Object Reference") (OtherComp :type "PrimitiveComponent Object Reference") (OtherBodyIndex :type Integer) (bFromSweep :type Boolean) (SweepResult :type "HitResult Structure (by ref)"))
  (bind _asthird_person_character (cast `/Game/Blueprints/Character/ThirdPersonCharacter` OtherActor))
  (`self.OpenDoor` _asthird_person_character))

(event `self.Box.OnComponentEndOverlap`
  (params (OverlappedComponent :type "PrimitiveComponent Object Reference") (OtherActor :type "Actor Object Reference") (OtherComp :type "PrimitiveComponent Object Reference") (OtherBodyIndex :type Integer))
  (cast `/Game/Blueprints/Character/ThirdPersonCharacter` OtherActor)
  (`self.CloseDoor`))

(event `OpenDoor`
  (params (Object :type "Object Object Reference"))
  (if (not (`self.InProgress`))
    (if (not (`self.IsOpen`))
      (bind (_direction _openprogression) (`Timeline|DoorTimeLine` :!via `PlayFromStart` :!label _label)
        (:`Update`
          (set `self.InProgress` true)
          (`SceneComponent.K2_SetRelativeRotation` (`self.DoorRotator`) (`KismetMathLibrary.MakeRotator` 0.0 0.0 (* _openprogression (`self.MaxDoorOpenAngle`))) false false))
        (:`Finished`
          (set `self.InProgress` false)
          (switch `ETimelineDirection` _direction
            (:`Forward`
              (set `self.IsOpen` true))
            (:`Backward`
              (set `self.IsOpen` false))))))))

(event `CloseDoor`
  (if (not (`self.InProgress`))
    (if (`self.IsOpen`)
      (goto _label :!via `ReverseFromEnd`))))

(fn `UserConstructionScript`
  (`SceneComponent.K2_AddRelativeRotation` (`self.DoorRotator`) (`KismetMathLibrary.MakeRotator` 0.0 0.0 (`KismetMathLibrary.SelectFloat` (`self.MaxDoorOpenAngle`) 0.0 (`self.IsOpen`))) false false))