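; BP_DoorBase_Lock is a lockable door variant that requires an Iron Key from the opener's backpack.
; OpenDoor passes straight to the parent when unlocked; when locked, it casts the passed object to ThirdPersonCharacter and checks the first ConsumableItems count in its BPBackpackComponent.
; A positive count unlocks the door, decrements that count and runs the parent open, while zero prints a key-needed message.
; CloseDoor simply defers to the parent.
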(event `self.OpenDoor`
  (params (Object :type "Object Object Reference"))
  (if (not (`self.IsLocked`))
    (`parent.OpenDoor` null :!label _label)
    (else
      (bind _asthird_person_character (cast `/Game/Blueprints/Character/ThirdPersonCharacter` Object))
      (bind _consumableitems (`/Game/Blueprints/Character/BP_BackpackComponent.ConsumableItems` (`/Game/Blueprints/Character/ThirdPersonCharacter.BP_BackpackComponent` _asthird_person_character)))
      (bind _output (`|GetArrayItem` _consumableitems))
      (`/Engine/EditorBlueprintResources/StandardMacros.CompareInt` _output
        (:`>`
          (set `self.IsLocked` false)
          (`KismetArrayLibrary.Array_Set` _consumableitems 0 (- _output 1))
          (goto _label))
        (:`==`
          (`KismetSystemLibrary.PrintString` "Iron Key Needed"))))))

(event `self.CloseDoor`
  (`parent.CloseDoor`))

(fn `UserConstructionScript`
  (`parent.UserConstructionScript`))