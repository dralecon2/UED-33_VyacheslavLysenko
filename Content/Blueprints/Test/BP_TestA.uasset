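; BP_TestA is a test actor that exercises container operations and a text label.
; On BeginPlay it adds to MyStuff, prints the CatList lookup for "CoolCat", then after a short delay adds to NewVar3 and prints its length.
; The construction script formats MyName into the TextRender component's text.
; The delta-time print and the DebugVisibility toggle for the text are disconnected and never run.
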(event `self.ReceiveBeginPlay`
  (`BlueprintSetLibrary.Set_Add` (`self.MyStuff`))
  (`KismetSystemLibrary.PrintString` (`KismetStringLibrary.Conv_IntToString` (`BlueprintMapLibrary.Map_Find` (`self.CatList`) "CoolCat")) true false (struct :`R` 0.257606 :`B` 0.317708 :`A` 1.0) 60.0)
  (`KismetSystemLibrary.Delay` 1.0)
  (`KismetArrayLibrary.Array_Add` (`self.NewVar_3`) true)
  (`KismetSystemLibrary.PrintString` (`KismetStringLibrary.Conv_IntToString` (`KismetArrayLibrary.Array_Length` (`self.NewVar_3`))) true false (struct :`R` 0.257606 :`B` 0.317708 :`A` 1.0) 5.0))

(event `self.ReceiveTick`
  (params (DeltaSeconds :type "Float (single-precision)")))

(fn `UserConstructionScript`
  (`TextRenderComponent.K2_SetText` (`self.TextRender`) (`|FormatText` "My name is {Name}" (`self.MyName`))))